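; BP_Lever is an interactable lever that opens a linked door.
; Its Interact event prints a message containing a display name, then calls OpenDoor directly on the TargetDoor reference.
; The graph comment describes handle rotation, state toggling and an Event Dispatcher broadcast, but none of these appear in the event logic.
; BeginPlay, overlap and Tick are disabled stubs, and the construction script only calls its parent.
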(event EventBeginPlay
  ;[0.15 0.15 0.15 0.5] H06 Salter/Kaldirac EventGraph: BPI_Interact cagrildiginda kolu cevirir (Roll rotation), durumunu tersine cevirir ve bagli cihazlara Event Dispatcher ile bildirir.
  (|CallParentFunction) ; This node is disabled and will not be called.\nDrag off pins to build functionality.
)

(event Collision|EventActorBeginOverlap
  (params (OtherActor :type Actor%20Object%20Reference))
  ;[0.15 0.15 0.15 0.5] H06 Salter/Kaldirac EventGraph: BPI_Interact cagrildiginda kolu cevirir (Roll rotation), durumunu tersine cevirir ve bagli cihazlara Event Dispatcher ile bildirir.
  (|CallParentFunction OtherActor) ; This node is disabled and will not be called.\nDrag off pins to build functionality.
)

(event EventTick
  (params (DeltaSeconds :type Float%20%28single-precision%29))
  ;[0.15 0.15 0.15 0.5] H06 Salter/Kaldirac EventGraph: BPI_Interact cagrildiginda kolu cevirir (Roll rotation), durumunu tersine cevirir ve bagli cihazlara Event Dispatcher ile bildirir.
  (|CallParentFunction DeltaSeconds) ; This node is disabled and will not be called.\nDrag off pins to build functionality.
)

(event EventInteract
  (params (Interactor :type Actor%20Object%20Reference))
  ;[0.15 0.15 0.15 0.5] H06 Salter/Kaldirac EventGraph: BPI_Interact cagrildiginda kolu cevirir (Roll rotation), durumunu tersine cevirir ve bagli cihazlara Event Dispatcher ile bildirir.
  (Development|PrintString (Utilities|String|Append "Etkilesim: " (Utilities|String|ToString(Text) (Variables|Default|GetDisplayName))))
  (Default|OpenDoor (Variables|Default|GetTargetDoor)))

(fn ConstructionScript
  (|CallParentFunction))