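; BP_Door is a door actor that slides its mesh up and down in response to linked pressure plates.
; At BeginPlay it binds to each plate's pressed and released dispatchers, tracking a pressed count.
; As written, it opens when the incremented count plus one equals the plate total, and any release while open closes it.
; MoveComponentTo animates the movement, and opening fires an OnOpened dispatcher immediately after that call.
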(event Custom|OpenDoor
  ;[0.15 0.15 0.15 0.5] H06 Kapi Mantigi EventGraph: Event Dispatcher veya BPI_Interact ile tetiklendiginde Timeline / VInterpTo ile acilma rotasyonunu gerceklestirir.
  (Variables|Default|SetbOpen true)
  (Components|MoveComponentTo (Variables|Default|GetDoorMesh) (Math|Vector|MakeVector 0.0 0.0 4.6e+02) (Math|Rotator|MakeRotator 0.0 0.0 0.0) false false 1.0 false)
  (Default|CallOnOpened))

(event Custom|CloseDoor
  ;[0.15 0.15 0.15 0.5] H06 Kapi Mantigi EventGraph: Event Dispatcher veya BPI_Interact ile tetiklendiginde Timeline / VInterpTo ile acilma rotasyonunu gerceklestirir.
  (Variables|Default|SetbOpen false)
  (Components|MoveComponentTo (Variables|Default|GetDoorMesh) (Math|Vector|MakeVector 0.0 0.0 1.5e+02) (Math|Rotator|MakeRotator 0.0 0.0 0.0) false false 1.0 false))

(event Custom|PlatePressed
  ;[0.15 0.15 0.15 0.5] H06 Kapi Mantigi EventGraph: Event Dispatcher veya BPI_Interact ile tetiklendiginde Timeline / VInterpTo ile acilma rotasyonunu gerceklestirir.
  (Variables|Default|SetPressedCount (+ (Variables|Default|GetPressedCount) (Class|KismetSystemLibrary|MakeLiteralInteger 1)))
  (if (== (+ (Variables|Default|GetPressedCount) (Class|KismetSystemLibrary|MakeLiteralInteger 1)) (Utilities|Array|Length (Variables|Default|GetPlates)))
    (CallFunction|OpenDoor)))

(event Custom|PlateReleased
  ;[0.15 0.15 0.15 0.5] H06 Kapi Mantigi EventGraph: Event Dispatcher veya BPI_Interact ile tetiklendiginde Timeline / VInterpTo ile acilma rotasyonunu gerceklestirir.
  (Variables|Default|SetPressedCount (Math|Integer|Max(Integer) 0 (- (Variables|Default|GetPressedCount) (Class|KismetSystemLibrary|MakeLiteralInteger 1))))
  (if (Variables|Default|GetbOpen)
    (CallFunction|CloseDoor)))

(event EventBeginPlay
  ;[0.15 0.15 0.15 0.5] H06 Kapi Mantigi EventGraph: Event Dispatcher veya BPI_Interact ile tetiklendiginde Timeline / VInterpTo ile acilma rotasyonunu gerceklestirir.
  (for _array_element (Variables|Default|GetPlates)
    (EventDispatchers|BindEventtoOnPlatePressed _array_element (delegate Custom|PlatePressed))
    (EventDispatchers|BindEventtoOnPlateReleased _array_element (delegate Custom|PlateReleased))))

(event Collision|EventActorBeginOverlap
  (params (OtherActor :type Actor%20Object%20Reference))
  ;[0.15 0.15 0.15 0.5] H06 Kapi Mantigi EventGraph: Event Dispatcher veya BPI_Interact ile tetiklendiginde Timeline / VInterpTo ile acilma rotasyonunu gerceklestirir.
)

(event EventTick
  (params (DeltaSeconds :type Float%20%28single-precision%29))
  ;[0.15 0.15 0.15 0.5] H06 Kapi Mantigi EventGraph: Event Dispatcher veya BPI_Interact ile tetiklendiginde Timeline / VInterpTo ile acilma rotasyonunu gerceklestirir.
)

(fn ConstructionScript)