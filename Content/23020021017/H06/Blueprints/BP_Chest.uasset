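; BP_Chest is an interactable chest actor that opens once when interacted with.
; Its Interact event prints the chest's DisplayName on every call, then checks an Opened flag.
; On the first interaction it sets the flag and uses MoveComponentTo to slide LidMesh to a raised relative location over half a second, with no rotation.
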(event EventBeginPlay
  (|CallParentFunction) ; This node is disabled and will not be called.\nDrag off pins to build functionality.
)

(event Collision|EventActorBeginOverlap
  (params (OtherActor :type Actor%20Object%20Reference))
  (|CallParentFunction OtherActor) ; This node is disabled and will not be called.\nDrag off pins to build functionality.
)

(event EventTick
  (params (DeltaSeconds :type Float%20%28single-precision%29))
  (|CallParentFunction DeltaSeconds) ; This node is disabled and will not be called.\nDrag off pins to build functionality.
)

(event EventInteract
  (params (Interactor :type Actor%20Object%20Reference))
  (Development|PrintString (Utilities|String|Append "Etkilesim: " (Utilities|String|ToString(Text) (Variables|Default|GetDisplayName))))
  (if (not (Variables|Default|GetbOpened))
    (Variables|Default|SetbOpened true)
    (Components|MoveComponentTo (Variables|Default|GetLidMesh) (Math|Vector|MakeVector 0.0 0.0 1.3e+02) (Math|Rotator|MakeRotator 0.0 0.0 0.0) false false 0.5 false)))

(fn ConstructionScript
  (|CallParentFunction))