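; BP_H06PlayerController is a player controller that lets the player interact with nearby actors by pressing E.
; On press, it gathers all actors implementing an interface and sends InteractMessage, passing the player pawn, to the first found within a fixed distance.
; The loop stops at that first match, which is not necessarily the nearest.
; A duplicate E handler runs the same search without acting, and disconnected leftover nodes remain.
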(event EventBeginPlay)

(event EventTick
  (params (DeltaSeconds :type Float%20%28single-precision%29)))

(event Input|KeyboardEvents|E
  (params (Key :type Key%20Structure)))

(event Input|KeyboardEvents|E
  (params (Key :type Key%20Structure))
  (:Pressed
    (bind _outactors (Actor|GetAllActorswithInterface 0))
    (bind _array_element (Utilities|Array|ForEachLoopwithBreak _outactors)
      (:LoopBody
        (if (<= (Transformation|GetDistanceTo _array_element (Game|Player|GetPlayerPawn 0)) 2.5e+02)
          _)))))

(event Input|KeyboardEvents|E
  (params (Key :type Key%20Structure))
  (bind _returnvalue (Game|Player|GetPlayerPawn 0))
  (:Pressed
    (bind _outactors (Actor|GetAllActorswithInterface 0))
    (bind _array_element (Utilities|Array|ForEachLoopwithBreak _outactors :!label _label)
      (:LoopBody
        (if (<= (Transformation|GetDistanceTo _array_element _returnvalue) 2.5e+02)
          (Class|BPIInteract|Interact(Message) _array_element _returnvalue)
          (goto _label Break))))))

(fn ConstructionScript)