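; Grid manager actor for a timed candy match-3 game, spawning a Size×Size board of randomly typed BP_PuzzleBlock actors.
; Selecting three same-type blocks in a straight adjacent line scores with a growing combo multiplier and respawns them; SwapMode treats two picks as a neighbor type swap.
; Looping timers reroll unselected blocks and count down to a win or loss against TargetScore.
; A HUD widget is created, but status updates use PrintString.
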(event EventBeginPlay
  (bind _self self)
  ;[0.15 0.15 0.15 0.5] H05 PuzzleGrid EventGraph: Oyun baslangicinda Grid i olusturur, zamanlayiciyi baslatir ve oyun dongusunu kontrol eder.
  (Development|PrintString "// [BASLANGIC]: Skor, sure ve kombo sifirlanir, UI olusturulur, izgara kurulur ve zamanlayicilar baslatilir.")
  (Development|PrintString "=== CANDY MATCH BASLADI! [Ana Mekanik: Swap / Yan Mekanik: Kombo Carpani] ===")
  (Variables|Default|SetScore 0)
  (Variables|Default|SetTimeLeft 60)
  (Variables|Default|SetComboMultiplier 1)
  (bind _returnvalue (UserInterface|CreateWidget "/Game/23020021017/H05/UI/W_PuzzleHUD.W_PuzzleHUD_C" (Game|GetPlayerController 0)))
  (Variables|Default|SetHud _returnvalue)
  (UserInterface|Viewport|AddtoViewport _returnvalue 0)
  (CallFunction|CreateGrid)
  (Utilities|Time|SetTimerbyFunctionName _self "RandomizeBlocks" 2.0 true)
  (Utilities|Time|SetTimerbyFunctionName _self "CountdownTick" 1.0 true)
  (CallFunction|UpdateHud))

(event Collision|EventActorBeginOverlap
  (params (OtherActor :type Actor%20Object%20Reference))
  ;[0.15 0.15 0.15 0.5] H05 PuzzleGrid EventGraph: Oyun baslangicinda Grid i olusturur, zamanlayiciyi baslatir ve oyun dongusunu kontrol eder.
)

(event EventTick
  (params (DeltaSeconds :type Float%20%28single-precision%29))
  ;[0.15 0.15 0.15 0.5] H05 PuzzleGrid EventGraph: Oyun baslangicinda Grid i olusturur, zamanlayiciyi baslatir ve oyun dongusunu kontrol eder.
)

(fn ConstructionScript)

(fn AreSameType
  (params (A :type Integer) (B :type Integer) (C :type Integer))
  (bind _blocks (Variables|Default|GetBlocks))
  (bind _output (Utilities|Array|Get(acopy) _blocks B))
  (bind _blocktype (Variables|/Game/23020021017/H05/Blueprints/BP_PuzzleBlock.BP_PuzzleBlock_C|GetBlockType _output))
  ;[0.15 0.15 0.15 0.5] H05 Tur Kontrolu: 3 blogun BlockType enum degerlerinin birbirine esit olup olmadigini dogrular.
  (return (and (== (Variables|/Game/23020021017/H05/Blueprints/BP_PuzzleBlock.BP_PuzzleBlock_C|GetBlockType (Utilities|Array|Get(acopy) (Variables|Default|GetBlocks) A)) _blocktype) (== _blocktype (Variables|/Game/23020021017/H05/Blueprints/BP_PuzzleBlock.BP_PuzzleBlock_C|GetBlockType (Utilities|Array|Get(acopy) (Variables|Default|GetBlocks) C))))))

(fn AreinLine
  (params (A :type Integer) (B :type Integer) (C :type Integer))
  (bind _returnvalue (Math|Integer|Min(Integer) A B))
  (bind _returnvalue_2 (Math|Integer|Max(Integer) A B))
  (bind _size (Variables|Default|GetSize))
  (bind _size_2 (Variables|Default|GetSize))
  (bind _returnvalue_3 (Math|Integer|%(Integer) B _size_2))
  (bind _returnvalue_4 (Math|Integer|Min(Integer) _returnvalue C))
  (bind _returnvalue_5 (Math|Integer|Max(Integer) _returnvalue_2 C))
  (bind _returnvalue_6 (/ B _size))
  ;[0.15 0.15 0.15 0.5] H05 Dogrultu Kontrolu: 3 blogun grid index lerini Satir ve Sutuna cevirerek ya ayni satirda ya da ayni sutunda ardisik oldugunu dogrular (capraz kabul edilmez).
  (return (or (and (and (== (/ A (Variables|Default|GetSize)) _returnvalue_6) (== _returnvalue_6 (/ C (Variables|Default|GetSize)))) (== (- _returnvalue_5 _returnvalue_4) (Class|KismetSystemLibrary|MakeLiteralInteger 2))) (and (and (== (Math|Integer|%(Integer) A (Variables|Default|GetSize)) _returnvalue_3) (== _returnvalue_3 (Math|Integer|%(Integer) C (Variables|Default|GetSize)))) (== (- _returnvalue_5 _returnvalue_4) (* (Class|KismetSystemLibrary|MakeLiteralInteger 2) (Variables|Default|GetSize)))))))

(fn CreateBlock
  (params (Row :type Integer) (Col :type Integer))
  (bind _self self)
  (bind _size (Variables|Default|GetSize))
  (bind _returnvalue (* Row _size))
  (bind _returnvalue_2 (+ _returnvalue Col))
  ;[0.15 0.15 0.15 0.5] H05 Blok Spawn: Belirtilen koordinatta BP_PuzzleBlock ornegi olusturur ve grid dizisine (Grid Array) kaydeder.
  (bind _returnvalue_3 (Game|SpawnActorfromClass "/Game/23020021017/H05/Blueprints/BP_PuzzleBlock.BP_PuzzleBlock_C" (Math|Transform|MakeTransform (+ (Transformation|GetActorLocation _self) (Math|Vector|MakeVector (* Row (Variables|Default|GetSpacing)) (* Col (Variables|Default|GetSpacing)) 0.0))) "Undefined" "MultiplyWithRoot" _self 0))
  (Variables|/Game/23020021017/H05/Blueprints/BP_PuzzleBlock.BP_PuzzleBlock_C|SetGridIndex _returnvalue_3 _returnvalue_2)
  (Variables|/Game/23020021017/H05/Blueprints/BP_PuzzleBlock.BP_PuzzleBlock_C|SetGrid _returnvalue_3 _self)
  (Default|AssignBlockType _returnvalue_3 (Math|Random|RandomIntegerinRange 0 2))
  (Utilities|Array|SetArrayElem (Variables|Default|GetBlocks) _returnvalue_2 _returnvalue_3 true)
  (return _returnvalue_3))

(fn BlockSelected
  (params (Block :type BP%20Puzzle%20Block%20Object%20Reference))
  (bind _activeblocks (Variables|Default|GetActiveBlocks))
  (bind _returnvalue (Utilities|Array|Length _activeblocks))
  ;[0.15 0.15 0.15 0.5] H05 Blok Secim Mantigi: Tiklanan blogu ActiveBlocks dizisine ekler. 3 blok secildiginde CheckMatch fonksiyonunu cagirir.
  (Development|PrintString "// [BLOK SECIMI & TETIKLEME]: 2 blok secilince Swap (Ana Mekanik), 3 blokta Match kontrol edilir.")
  (if (not (or (Variables|Default|GetbBreaking) (Variables|Default|GetbGameOver)))
    (Utilities|Array|AddUnique (Variables|Default|GetActiveBlocks) (Variables|/Game/23020021017/H05/Blueprints/BP_PuzzleBlock.BP_PuzzleBlock_C|GetGridIndex Block))
    (if (== _returnvalue (Class|KismetSystemLibrary|MakeLiteralInteger 3))
      (CallFunction|CheckMatch)
      (elif (and (Variables|Default|GetbSwapMode) (== _returnvalue (Class|KismetSystemLibrary|MakeLiteralInteger 2)))
        (CallFunction|SwapBlocks self (Utilities|Array|Get(acopy) (Variables|Default|GetActiveBlocks)) (Utilities|Array|Get(acopy) (Variables|Default|GetActiveBlocks) 1))))))

(fn ClearSelection
  ;[0.15 0.15 0.15 0.5] H05 Secimi Temizle: Secilen bloklarin secim gorselini kaldirir ve ActiveBlocks listesini bosaltir.
  (Development|PrintString "// [SECIMI TEMIZLE]: Secili sekerleri serbest birak ve secim listesini sifirla.")
  (for _array_element (Variables|Default|GetActiveBlocks)
    (Default|MakeSelectable (Utilities|Array|Get(acopy) (Variables|Default|GetBlocks) _array_element)))
  (Utilities|Array|Clear (Variables|Default|GetActiveBlocks)))

(fn EndGame
  ;[0.15 0.15 0.15 0.5] H05 Oyun Bitisi: Sure bittiginde veya hamle kalmadiginda oyunu sonlandirir ve skor tablosunu sunar.
  (Development|PrintString "// [KAYBETME KOSULU]: Sure doldu ve hedef puana ulasilamadi! Oyun sona erer.")
  (Variables|Default|SetbGameOver true)
  (Variables|Default|SetbGameWon false)
  (Utilities|Time|ClearandInvalidateTimerbyHandle (Variables|Default|GetRandomizeTimer))
  (Utilities|Time|ClearandInvalidateTimerbyHandle (Variables|Default|GetCountdownTimer))
  (Development|PrintString "SURE BITTI - KAYBETTINIZ! 😢 Hedef: 300 Puan")
  (CallFunction|UpdateHud))

(fn UpdateHud
  (bind _score (Variables|Default|GetScore))
  (bind _timeleft (Variables|Default|GetTimeLeft))
  (bind _combomultiplier (Variables|Default|GetComboMultiplier))
  ;[0.15 0.15 0.15 0.5] H05 Arayuz Guncelleme: Kalan sure, mevcut skor ve hedef puan bilgilerini ekrandaki UI a aktarir.
  (if (Variables|Default|GetbGameWon)
    (Development|PrintString (Utilities|String|Append (Utilities|String|Append (Utilities|String|Append (Utilities|String|Append (Utilities|String|Append "🎉 [KAZANDINIZ!] Tebrikler! Skor: " (Utilities|String|ToString(Integer) _score)) " / 300 | Kalan Sure: ") (Utilities|String|ToString(Integer) _timeleft)) " sn | Kombo: x") (Utilities|String|ToString(Integer) _combomultiplier)))
    (elif (Variables|Default|GetbGameOver)
      (Development|PrintString (Utilities|String|Append (Utilities|String|Append "😢 [KAYBETTINIZ!] Sure Bitti! Skorunuz: " (Utilities|String|ToString(Integer) _score)) " / 300"))
      (else
        (Development|PrintString (Utilities|String|Append (Utilities|String|Append (Utilities|String|Append (Utilities|String|Append (Utilities|String|Append "[CANDY] Hedef: 300 | Skor: " (Utilities|String|ToString(Integer) _score)) " | Sure: ") (Utilities|String|ToString(Integer) _timeleft)) " sn | Kombo: x") (Utilities|String|ToString(Integer) _combomultiplier)))))))

(fn RefillBlocks
  ;[0.15 0.15 0.15 0.5] H05 Grid Doldurma: Kirilan bloklarin ustundeki bloklari asagi kaydirir ve en ust satira yeni rastgele bloklar uretir.
  (for _array_element (Variables|Default|GetActiveBlocks)
    (CallFunction|CreateBlock (/ _array_element (Variables|Default|GetSize)) (Math|Integer|%(Integer) _array_element (Variables|Default|GetSize))))
  (Utilities|Array|Clear (Variables|Default|GetActiveBlocks))
  (Variables|Default|SetbBreaking false)
  (Utilities|Time|UnpauseTimerbyHandle (Variables|Default|GetRandomizeTimer)))

(fn CheckMatch
  (bind _self self)
  (bind _activeblocks (Variables|Default|GetActiveBlocks))
  (bind _output (Utilities|Array|Get(acopy) _activeblocks))
  (bind _output_2 (Utilities|Array|Get(acopy) _activeblocks 1))
  (bind _output_3 (Utilities|Array|Get(acopy) _activeblocks 2))
  ;[0.15 0.15 0.15 0.5] H05 Eslesme Kontrolu: Secilen 3 blogun ayni turde olup olmadigini (AreSameType) ve ayni dogrultuda olup olmadigini (AreInLine) kontrol eder. Eslesirse BreakMatched cagirilir.
  (Development|PrintString "// [ESLESME KONTROLU]: Secilen 3 seker ayni turde ve ayni satir/sutunda mi kontrol edilir.")
  (bind _same (CallFunction|AreSameType _self _output _output_2 _output_3))
  (bind _inline (CallFunction|AreinLine _self _output _output_2 _output_3))
  (if (and _same _inline)
    (CallFunction|BreakMatched)
    (else
      (CallFunction|ClearSelection))))

(fn BreakMatched
  ;[0.15 0.15 0.15 0.5] H05 Eslesenleri Kirma: Eslesen 3 blogu kirar (BreakBlock), skoru artirir ve bosalan yerler icin RefillBlocks cagirir.
  (Development|PrintString "// [YAN MEKANIK - KOMBO CARPANI]: Puan hesabi (+30 * Kombo). 300 puanda WinGame tetiklenir.")
  (Variables|Default|SetbBreaking true)
  (Utilities|Time|PauseTimerbyHandle (Variables|Default|GetRandomizeTimer))
  (Variables|Default|SetScore (+ (Variables|Default|GetScore) (* (Class|KismetSystemLibrary|MakeLiteralInteger 30) (Variables|Default|GetComboMultiplier))))
  (Variables|Default|SetComboMultiplier (+ (Variables|Default|GetComboMultiplier) (Class|KismetSystemLibrary|MakeLiteralInteger 1)))
  (Development|PrintString "ESLESME BASARILI! KOMBO ARTIRILDI!")
  (CallFunction|UpdateHud)
  (if (>= (Variables|Default|GetScore) (Variables|Default|GetTargetScore))
    (CallFunction|WinGame))
  (for _array_element (Variables|Default|GetActiveBlocks)
    (Default|BreakBlock (Utilities|Array|Get(acopy) (Variables|Default|GetBlocks) _array_element)))
  (CallFunction|RefillBlocks))

(fn CountdownTick
  ;[0.15 0.15 0.15 0.5] H05 Geri Sayim: Oyun suresini her saniye 1 azaltir; sure bittiginde EndGame tetikler.
  (Development|PrintString "// [GERI SAYIM & SURE]: Sure 1 sn azalir. Sure bitince kazanma/kaybetme kontrol edilir.")
  (Variables|Default|SetTimeLeft (- (Variables|Default|GetTimeLeft) (Class|KismetSystemLibrary|MakeLiteralInteger 1)))
  (CallFunction|UpdateHud)
  (if (<= (Variables|Default|GetTimeLeft) (Class|KismetSystemLibrary|MakeLiteralInteger))
    (if (>= (Variables|Default|GetScore) (Variables|Default|GetTargetScore))
      (CallFunction|WinGame)
      (else
        (CallFunction|EndGame)))))

(fn RandomizeBlocks
  ;[0.15 0.15 0.15 0.5] H05 Grid Karistirma: Hic hamle kalmadiginda tum bloklarin turlerini yeniden rastgele dagitir.
  (Development|PrintString "// [RASTGELE BLOK DEGISIMI]: Her 2 saniyede secili olmayan sekerlerin tipi rastgele degisir.")
  (for _array_element (Variables|Default|GetBlocks)
    (if (not (Variables|/Game/23020021017/H05/Blueprints/BP_PuzzleBlock.BP_PuzzleBlock_C|GetbIsActive _array_element))
      (Default|AssignBlockType _array_element (Math|Random|RandomIntegerinRange 0 2)))))

(fn CreateGrid
  ;[0.15 0.15 0.15 0.5] H05 Grid Olusturma: Belirlenen Satir x Sutun (4x4) boyutlarinda matematiksel olarak blok konumlarini hesaplar ve Spawn eder.
  (for _index (range 0 (- (Variables|Default|GetSize) (Class|KismetSystemLibrary|MakeLiteralInteger 1)))
    (for _index_2 (range 0 (- (Variables|Default|GetSize) (Class|KismetSystemLibrary|MakeLiteralInteger 1)))
      (CallFunction|CreateBlock _index _index_2))))

(fn SwapBlocks
  (params (IndexA :type Integer) (IndexB :type Integer))
  (bind _blocks (Variables|Default|GetBlocks))
  (bind _output (Utilities|Array|Get(acopy) _blocks IndexB))
  (bind _output_2 (Utilities|Array|Get(acopy) _blocks IndexA))
  ;[0.15 0.15 0.15 0.5] H05 Blok Degisimi: Iki komsu blogun grid dizisindeki index lerini ve sahnedeki konumlarini takas eder.
  (Development|PrintString "// [ANA MEKANIK - SWAP]: Komsu 2 sekerin satir/sutun mesafesini kontrol et ve yer degistir.")
  (if (== (+ (Math|Integer|Absolute(Integer) (- (/ IndexA (Variables|Default|GetSize)) (/ IndexB (Variables|Default|GetSize)))) (Math|Integer|Absolute(Integer) (- (Math|Integer|%(Integer) IndexA (Variables|Default|GetSize)) (Math|Integer|%(Integer) IndexB (Variables|Default|GetSize))))) (Class|KismetSystemLibrary|MakeLiteralInteger 1))
    (Default|AssignBlockType _output_2 (Variables|/Game/23020021017/H05/Blueprints/BP_PuzzleBlock.BP_PuzzleBlock_C|GetBlockType _output))
    (Default|AssignBlockType _output (Variables|/Game/23020021017/H05/Blueprints/BP_PuzzleBlock.BP_PuzzleBlock_C|GetBlockType _output_2))
    (Development|PrintString "SWAP BASARILI! Komsu sekerler yer degistirdi.")
    (CallFunction|ClearSelection)
    (return true)
    (else
      (Development|PrintString "GECERSIZ HAMLE! Sadece komsu sekerler yer degistirebilir.")
      (CallFunction|ClearSelection)
      (return false))))

(fn WinGame
  ;[0.15 0.15 0.15 0.5] H05 Kazanma Durumu: Hedef skora ulasildiginda oyunu durdurur ve zafer ekranini gosterir.
  (Development|PrintString "// [KAZANMA KOSULU]: Hedef skora (300) ulasildi! Sayaçlar durdurulur ve oyun zaferle biter.")
  (Variables|Default|SetbGameOver true)
  (Variables|Default|SetbGameWon true)
  (Utilities|Time|ClearandInvalidateTimerbyHandle (Variables|Default|GetRandomizeTimer))
  (Utilities|Time|ClearandInvalidateTimerbyHandle (Variables|Default|GetCountdownTimer))
  (Development|PrintString "🎉 TEBRIKLER! OYUNU KAZANDINIZ! HEDEF SKOR (300) TAMAMLANDI! 🎉")
  (CallFunction|UpdateHud))