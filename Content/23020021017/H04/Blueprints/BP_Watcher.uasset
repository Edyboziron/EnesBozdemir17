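; BP_Watcher is a sentry actor that detects the player with a vision cone and shows whether it is alerted.
; Each Tick it draws a 45-degree debug cone, then calls CanSeePlayer, which combines a ViewDistance check with a forward-vector dot product against ConeDot.
; The result swaps the Body material between alert and calm, printing a "seen" message while detected.
; Detection uses no line trace, so obstacles do not block sight.
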(event EventBeginPlay
  ;[0.15 0.15 0.15 0.5] H04 Gozcu EventGraph: Her Tick te DrawDebugCone ile 45 derecelik gorus konisini cizer. CanSeePlayer True ise alert materyaline (MI_WatcherAlert) gecer, degilse calm materyaline doner.
)

(event Collision|EventActorBeginOverlap
  (params (OtherActor :type Actor%20Object%20Reference))
  ;[0.15 0.15 0.15 0.5] H04 Gozcu EventGraph: Her Tick te DrawDebugCone ile 45 derecelik gorus konisini cizer. CanSeePlayer True ise alert materyaline (MI_WatcherAlert) gecer, degilse calm materyaline doner.
)

(event EventTick
  (params (DeltaSeconds :type Float%20%28single-precision%29))
  ;[0.15 0.15 0.15 0.5] H04 Gozcu EventGraph: Her Tick te DrawDebugCone ile 45 derecelik gorus konisini cizer. CanSeePlayer True ise alert materyaline (MI_WatcherAlert) gecer, degilse calm materyaline doner.
  (Class|KismetSystemLibrary|DrawDebugConeinDegrees (+ (Transformation|GetActorLocation) (Math|Vector|MakeVector 0.0 0.0 185.0)) (Transformation|GetActorForwardVector) (Variables|Default|GetViewDistance) 45.0 45.0 24 "(R=1.0,G=1.0,B=0.0,A=1.0)" 0.0 1.5 "World")
  (bind _seen (CallFunction|CanSeePlayer))
  (if _seen
    (Rendering|Material|SetMaterial (Variables|Default|GetBody) 0 "/Game/23020021017/H04/Materials/MI_WatcherAlert.MI_WatcherAlert")
    (Development|PrintString "GÖRÜLDÜN!" true true "(R=1.0,G=0.0,B=0.0,A=1.0)" 0.0 "Gozcu")
    (else
      (Rendering|Material|SetMaterial (Variables|Default|GetBody) 0 "/Game/23020021017/H04/Materials/MI_WatcherCalm.MI_WatcherCalm"))))

(fn ConstructionScript)

(fn CanSeePlayer
  (bind _returnvalue (Game|GetPlayerCharacter 0))
  (bind _returnvalue_2 (Transformation|GetActorLocation))
  (bind _returnvalue_3 (Transformation|GetActorForwardVector))
  (bind _returnvalue_4 (Transformation|GetActorLocation _returnvalue))
  (bind _returnvalue_5 (Math|Vector|GetUnitDirection(Vector) _returnvalue_2 _returnvalue_4))
  (bind _returnvalue_6 (Math|Vector|DotProduct _returnvalue_3 _returnvalue_5))
  ;[0.15 0.15 0.15 0.5] H04 CanSeePlayer: Oyuncuya olan yon vektorunu normalize eder, Forward Vector ile Dot Product (A.B >= cos(45)=0.707) ve mesafe kontrolu yapar.
  (Variables|Default|SetDotValue _returnvalue_6)
  (return (and (< (Transformation|GetDistanceTo _returnvalue) (Variables|Default|GetViewDistance)) (> _returnvalue_6 (Variables|Default|GetConeDot)))))