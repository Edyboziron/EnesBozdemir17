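; BP_MaterialDisplay is a material showcase Blueprint that cycles the look of its Display component when E is pressed.
; BeginPlay calls EnableInput using the first player controller, intended for the E key event.
; A looping, sequential MultiGate steps through gold, copper and nickel material instances on the first material slot.
; Each switch prints the material's Turkish name on screen.
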(event EventBeginPlay
  (Input|EnableInput (Game|GetPlayerController 0) 0))

(event Collision|EventActorBeginOverlap
  (params (OtherActor :type Actor%20Object%20Reference)))

(event EventTick
  (params (DeltaSeconds :type Float%20%28single-precision%29)))

(event Input|KeyboardEvents|E
  (params (Key :type Key%20Structure)))

(event Input|KeyboardEvents|E
  (params (Key :type Key%20Structure))
  (:Pressed
    (Utilities|FlowControl|MultiGate false true -1
      (:Out%200
        (Rendering|Material|SetMaterial (Variables|Default|GetDisplay) 0 "/Game/23020021017/H03/Materials/MI_Gold.MI_Gold")
        (Development|PrintString "Materyal: Altin"))
      (:Out%201
        (Rendering|Material|SetMaterial (Variables|Default|GetDisplay) 0 "/Game/23020021017/H03/Materials/MI_Copper.MI_Copper")
        (Development|PrintString "Materyal: Bakir"))
      (:Out%202
        (Rendering|Material|SetMaterial (Variables|Default|GetDisplay) 0 "/Game/23020021017/H03/Materials/MI_Nickel.MI_Nickel")
        (Development|PrintString "Materyal: Nikel")))))

(fn ConstructionScript)