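; BP_Mine is a mine actor that launches an overlapping Character straight upward, hides its mesh and prints an explosion message.
; Actor overlap passes through a DoOnce before the Character cast, so any first overlapping actor uses up the trigger.
; BeginPlay enables input, and pressing R re-shows the mesh with a re-arm message but does not reset the DoOnce.
; An unreachable copy of the launch chain remains in the graph.
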(event EventBeginPlay
  (Input|EnableInput (Game|GetPlayerController 0) 0))

(event Collision|EventActorBeginOverlap
  (params (OtherActor :type Actor%20Object%20Reference))
  (Utilities|FlowControl|DoOnce false
    (:Completed
      (bind _ascharacter (Utilities|Casting|CastToCharacter OtherActor))
      (Character|LaunchCharacter _ascharacter (Math|Vector|MakeVector 0.0 0.0 1.2e+03) false true)
      (Rendering|SetVisibility (Variables|Default|GetMineMesh) false false)
      (Development|PrintString "Mayin patladi!"))))

(event EventTick
  (params (DeltaSeconds :type Float%20%28single-precision%29)))

(event Input|KeyboardEvents|R
  (params (Key :type Key%20Structure))
  (:Pressed
    (Rendering|SetVisibility (Variables|Default|GetMineMesh) true false)
    (Development|PrintString "Mayin yeniden kuruldu.")))

(fn ConstructionScript)