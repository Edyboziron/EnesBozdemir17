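; Loot chest actor that rolls a seeded random item, rarity and power when the player presses E within range.
; BeginPlay seeds a random stream, applies the chest material and enables input.
; OpenChest derives power from weighted rarity, base power and a level-capped roll, tints base and lid from grey to gold by power, then prints the result.
; Nothing prevents repeated opening; each press advances the stream.
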(event EventBeginPlay
  (Variables|Default|SetStream (Math|Random|MakeRandomStream (Variables|Default|GetSeed)))
  (Rendering|Material|SetMaterial (Variables|Default|GetChestBase) 0 "/Game/23020021017/H03/Materials/MI_Chest.MI_Chest")
  (Rendering|Material|SetMaterial (Variables|Default|GetChestLid) 0 "/Game/23020021017/H03/Materials/MI_Chest.MI_Chest")
  (Input|EnableInput (Game|GetPlayerController 0)))

(event Input|KeyboardEvents|E
  (params (Key :type Key%20Structure))
  (:Pressed
    (if (<= (Transformation|GetDistanceTo (Game|GetPlayerCharacter 0)) 3e+02)
      (CallFunction|OpenChest))))

(fn ConstructionScript)

(fn RollRarity
  (bind _stream (Variables|Default|GetStream))
  (bind _returnvalue (Math|Random|RandomFloatfromStream _stream))
  (if (< _returnvalue (Math|Float|MakeLiteralFloat 0.6))
    (return "Common")
    (elif (< _returnvalue (Math|Float|MakeLiteralFloat 0.9))
      (return "Rare")
      (else
        (return "Legendary")))))

(fn RarityBonus
  (params (InRarity :type String))
  (return (select (Utilities|Enum|Equal(Enum) InRarity "Common") (Math|Float|MakeLiteralFloat 0.0) (select (Utilities|Enum|Equal(Enum) InRarity "Rare") (Math|Float|MakeLiteralFloat 0.5) (Math|Float|MakeLiteralFloat 1.5)))))

(fn CalculatePower
  (params (Base :type Float%20%28double-precision%29) (Bonus :type Float%20%28double-precision%29) (Roll :type Integer))
  (return (+ (* Base (+ (Math|Float|MakeLiteralFloat 1.0) Bonus)) Roll)))

(fn OpenChest
  (bind _returnvalue (CallFunction|RollRarity))
  (Variables|Default|SetRarity _returnvalue)
  (bind _returnvalue_2 (CallFunction|RarityBonus _returnvalue))
  (bind _returnvalue_3 (CallFunction|CalculatePower (Variables|Default|GetBasePower) _returnvalue_2 (Math|Random|RandomIntegerinRangefromStream (Variables|Default|GetStream) 0 (Variables|Default|GetChestLevel))))
  (Variables|Default|SetPower _returnvalue_3)
  (Rendering|Material|SetVectorParameterValueonMaterials (Variables|Default|GetChestBase) "Color" (Math|Conversions|ToVector(LinearColor) (Math|Color|Lerp(LinearColor) (Utilities|Struct|MakeLinearColor 0.25 0.25 0.25 1.0) (Utilities|Struct|MakeLinearColor 1.0 0.8 0.1 1.0) (Math|Float|MapRangeClamped _returnvalue_3 1e+01 4e+01 0.0 1.0))))
  (Rendering|Material|SetVectorParameterValueonMaterials (Variables|Default|GetChestLid) "Color" (Math|Conversions|ToVector(LinearColor) (Math|Color|Lerp(LinearColor) (Utilities|Struct|MakeLinearColor 0.25 0.25 0.25 1.0) (Utilities|Struct|MakeLinearColor 1.0 0.8 0.1 1.0) (Math|Float|MapRangeClamped _returnvalue_3 1e+01 4e+01 0.0 1.0))))
  (Development|PrintString (Utilities|String|Append (Utilities|String|Append (Utilities|String|Append (Utilities|String|Append (.OutItem (Utilities|Array|RandomFromStream (Variables|Default|GetItems) (Variables|Default|GetStream))) " (") _returnvalue) ") — Guc: ") (Utilities|String|ToString(Float) _returnvalue_3)) true true "(R=0.000000,G=0.660000,B=1.000000,A=1.000000)" 5.0))