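; BP_HealthStation is a healing station that restores the player character's health over time while something overlaps it.
; Begin and end overlap open and close a Gate, which starts closed and passes Tick into Heal.
; Heal casts player 0 to BP_ThirdPersonCharacter, adds health at a fixed rate scaled by delta time, caps it at MaxHealth and prints it.
; The overlap events do not check which actor triggers them.
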(event EventBeginPlay)

(event Collision|EventActorBeginOverlap
  (params (OtherActor :type Actor%20Object%20Reference))
  (Utilities|FlowControl|Gate true ; enters at Open
    (:Exit
      (CallFunction|Heal (stale EventTick DeltaSeconds)))))

(event EventTick
  (params (DeltaSeconds :type Float%20%28single-precision%29))
  (Utilities|FlowControl|Gate true
    (:Exit
      (CallFunction|Heal DeltaSeconds))))

(event Collision|EventActorEndOverlap
  (params (OtherActor :type Actor%20Object%20Reference))
  (Utilities|FlowControl|Gate true ; enters at Close
    (:Exit
      (CallFunction|Heal (stale EventTick DeltaSeconds)))))

(fn ConstructionScript)

(fn Heal
  (params (DeltaSeconds :type Float%20%28double-precision%29))
  (bind _asbp_third_person_character (Utilities|Casting|CastToBP_ThirdPersonCharacter (Game|GetPlayerCharacter 0)))
  (Variables|/Game/ThirdPerson/Blueprints/BP_ThirdPersonCharacter.BP_ThirdPersonCharacter_C|SetHealth _asbp_third_person_character (select (< (+ (Variables|/Game/ThirdPerson/Blueprints/BP_ThirdPersonCharacter.BP_ThirdPersonCharacter_C|GetHealth _asbp_third_person_character) (* (Math|Float|MakeLiteralFloat 25.0) DeltaSeconds)) (Variables|/Game/ThirdPerson/Blueprints/BP_ThirdPersonCharacter.BP_ThirdPersonCharacter_C|GetMaxHealth _asbp_third_person_character)) (+ (Variables|/Game/ThirdPerson/Blueprints/BP_ThirdPersonCharacter.BP_ThirdPersonCharacter_C|GetHealth _asbp_third_person_character) (* (Math|Float|MakeLiteralFloat 25.0) DeltaSeconds)) (Variables|/Game/ThirdPerson/Blueprints/BP_ThirdPersonCharacter.BP_ThirdPersonCharacter_C|GetMaxHealth _asbp_third_person_character)))
  (Development|PrintString (Utilities|String|Append "Can: " (Utilities|String|ToString(Float) (select (< (+ (Variables|/Game/ThirdPerson/Blueprints/BP_ThirdPersonCharacter.BP_ThirdPersonCharacter_C|GetHealth _asbp_third_person_character) (* (Math|Float|MakeLiteralFloat 25.0) DeltaSeconds)) (Variables|/Game/ThirdPerson/Blueprints/BP_ThirdPersonCharacter.BP_ThirdPersonCharacter_C|GetMaxHealth _asbp_third_person_character)) (+ (Variables|/Game/ThirdPerson/Blueprints/BP_ThirdPersonCharacter.BP_ThirdPersonCharacter_C|GetHealth _asbp_third_person_character) (* (Math|Float|MakeLiteralFloat 25.0) DeltaSeconds)) (Variables|/Game/ThirdPerson/Blueprints/BP_ThirdPersonCharacter.BP_ThirdPersonCharacter_C|GetMaxHealth _asbp_third_person_character)))) true true "(R=0.000000,G=0.660000,B=1.000000,A=1.000000)" 2.0 "Can"))