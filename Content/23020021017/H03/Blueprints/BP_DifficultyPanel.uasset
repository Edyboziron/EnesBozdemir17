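; Difficulty selection actor that maps number keys 1–4 to Easy, Normal, Hard and Nightmare presets with Turkish labels.
; BeginPlay calls EnableInput with the first player controller, and each key passes a level index to ApplyDifficulty.
; ApplyDifficulty switches on the index and only prints the difficulty name and enemy count, or an invalid-difficulty message, without spawning or storing anything.
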(event EventBeginPlay
  (Input|EnableInput (Game|GetPlayerController 0) 0))

(event Collision|EventActorBeginOverlap
  (params (OtherActor :type Actor%20Object%20Reference)))

(event EventTick
  (params (DeltaSeconds :type Float%20%28single-precision%29)))

(event Input|KeyboardEvents|1
  (params (Key :type Key%20Structure)))

(event Input|KeyboardEvents|2
  (params (Key :type Key%20Structure)))

(event Input|KeyboardEvents|3
  (params (Key :type Key%20Structure)))

(event Input|KeyboardEvents|4
  (params (Key :type Key%20Structure)))

(event Input|KeyboardEvents|1
  (params (Key :type Key%20Structure))
  (:Pressed
    (CallFunction|ApplyDifficulty)))

(event Input|KeyboardEvents|2
  (params (Key :type Key%20Structure))
  (:Pressed
    (CallFunction|ApplyDifficulty 1)))

(event Input|KeyboardEvents|3
  (params (Key :type Key%20Structure))
  (:Pressed
    (CallFunction|ApplyDifficulty 2)))

(event Input|KeyboardEvents|4
  (params (Key :type Key%20Structure))
  (:Pressed
    (CallFunction|ApplyDifficulty 3)))

(fn ConstructionScript)

(fn ApplyDifficulty
  (params (Level :type Integer))
  (switch int Level
    (:Default
      (Development|PrintString "Gecersiz zorluk"))
    (:0
      (Development|PrintString "Kolay: 5 dusman"))
    (:1
      (Development|PrintString "Normal: 10 dusman"))
    (:2
      (Development|PrintString "Zor: 15 dusman"))
    (:3
      (Development|PrintString "Kabus: 25 dusman"))))